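; Collectable crystal actor that gets absorbed into the player pawn on overlap, then destroys itself; no score or inventory logic is present.
; An IsPlayer macro gates the overlap, then the start location, scale and point light intensity are cached.
; A timeline's separate alpha tracks lerp the crystal toward the pawn's live position, shrink it to zero and fade its light before destruction.
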(event `self.ReceiveActorBeginOverlap`
  (params (OtherActor :type "Actor Object Reference"))
  (`self.IsPlayer` OtherActor
    (:`True`
      (`self.Object Start Location`)
      (bind (_direction _alpha1 _scale _light) (`Timeline|TL_BlendAlpha`)
        (:`Update`
          (`self.Change Location` _alpha1)
          (`self.Change Scale ` _scale)
          (`self.Change Light ` _light))
        (:`Finished`
          (`self.K2_DestroyActor`))))))

(fn `Change Light`
  (`LightComponent.SetIntensity` (`self.PointLight`) (`KismetMathLibrary.Lerp` (`self.LerpStartLight`))))

(fn `Change Light `
  (params (Alpha :type "Float (double-precision)"))
  (`LightComponent.SetIntensity` (`self.PointLight`) (`KismetMathLibrary.Lerp` (`self.LerpStartLight`) 0.0 Alpha)))

(fn `Change Location`
  (params (Alpha :type "Float (double-precision)"))
  (`self.K2_SetActorLocation` (`KismetMathLibrary.VLerp` (`self.LerpStartLocation`) (`self.K2_GetActorLocation` (`GameplayStatics.GetPlayerPawn` 0)) Alpha)))

(fn `Change Scale`
  (`self.K2_SetActorLocation` (`KismetMathLibrary.VLerp` (`self.Lerp Start Scale`))))

(fn `Change Scale `
  (params (Alpha :type "Float (double-precision)"))
  (`self.SetActorScale3D` (`KismetMathLibrary.VLerp` (`self.Lerp Start Scale`) (0.0 0.0 0.0) Alpha)))

(fn `Object Start Location`
  (set `self.LerpStartLocation` (`self.K2_GetActorLocation`))
  (set `self.Lerp Start Scale` (`self.GetActorScale3D`))
  (set `self.LerpStartLight` (`LightComponentBase.Intensity` (`self.PointLight`))))

(fn `UserConstructionScript`)