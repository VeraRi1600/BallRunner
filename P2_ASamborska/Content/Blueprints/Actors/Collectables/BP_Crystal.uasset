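; BP_Crystal is a collectable crystal actor that reacts when the player pawn overlaps it.
; On overlap it stores its location and plays a timeline that sets its position each update by lerping from that point toward the pawn's current location.
; The lerp alpha is a constant zero, so the crystal stays at its start point.
; It destroys itself when the timeline finishes, with no reward logic.
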(event `self.ReceiveActorBeginOverlap`
  (params (OtherActor :type "Actor Object Reference"))
  (if (== OtherActor (`GameplayStatics.GetPlayerPawn` 0))
    (set `self.LerpStartLocation` (`self.K2_GetActorLocation`))
    (`Timeline|Timeline_0`
      (:`Update`
        (`self.K2_SetActorLocation` (`KismetMathLibrary.VLerp` (`self.LerpStartLocation`) (`self.K2_GetActorLocation` (`GameplayStatics.GetPlayerPawn` 0)))))
      (:`Finished`
        (`self.K2_DestroyActor`)))))

(fn `UserConstructionScript`)